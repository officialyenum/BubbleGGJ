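; Master food pickup whose FoodItem key selects its sprite and heal amount from lookup maps, with the sprite set in the Construction Script.
; On overlap it clears Consumable, then heals Player-tagged actors through BPC_StatComponent, plays effect and sound, hides itself and starts a respawn timer.
; Reconsumeable restores visibility and Consumable.
; A non-player overlap also clears Consumable but starts no timer.
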(event `self.ReceiveActorBeginOverlap`
  (params (OtherActor :type "Actor Object Reference"))
  (`self.Heal` OtherActor))

(fn `Heal`
  (params (InputPin :type "Actor Object Reference"))
  (bind _value (`BlueprintMapLibrary.Map_Find` (`self.FoodHealth`) (`self.FoodItem`)))
  (if (`self.Consumable`)
    (set `self.Consumable` false)
    (if (`self.ActorHasTag` InputPin "Player")
      (`/Game/Characters/BPC_StatComponent.Heal` (`self.GetComponentByClass` InputPin "/Game/Characters/BPC_StatComponent.BPC_StatComponent_C") _value)
      (`|ExecutionSequence`
        (:`then_0`
          (`NiagaraFunctionLibrary.SpawnSystemAtLocation` "/Game/Effects/SlamEffect.SlamEffect" (`self.K2_GetActorLocation`) (struct) (1.0 1.0 1.0) true true "AutoRelease")
          (`GameplayStatics.PlaySound2D` "/Game/Assets/sounds/NomNom__1__Cue.NomNom__1__Cue" 1.0 1.0 0.0 null null)
          (`SceneComponent.SetHiddenInGame` (`self.PaperFlipbook`) true false)
          (`SceneComponent.SetHiddenInGame` (`self.PaperSprite`) true false)
          (`SceneComponent.SetHiddenInGame` (`self.Sphere`) true false)
          (`KismetSystemLibrary.K2_SetTimerDelegate` (`|CreateDelegate` :!event `Reconsumeable`) (`self.ReconsumableTimer`)))
        (:`then_1`
          (`KismetSystemLibrary.PrintString` (`KismetStringLibrary.Conv_IntToString` _value)))))))

(fn `Reconsumeable`
  (set `self.Consumable` true)
  (`SceneComponent.SetHiddenInGame` (`self.PaperSprite`) false false)
  (`SceneComponent.SetHiddenInGame` (`self.PaperFlipbook`) false false)
  (`SceneComponent.SetHiddenInGame` (`self.Sphere`) false false))

(fn `UserConstructionScript`
  (`PaperSpriteComponent.SetSprite` (`self.PaperSprite`) (`BlueprintMapLibrary.Map_Find` (`self.PossibleSprites`) (`self.FoodItem`))))