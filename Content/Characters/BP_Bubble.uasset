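; BP_Bubble is the player bubble, which steadily floats upward and sinks while the IA_Drop input is held.
; BeginPlay adds the Enhanced Input mapping context, starts health and runs a looping timer, replacing Tick, that offsets Z by AccelSpeed scaled by the timer interval.
; BPC_StatComponent owns health, with changes forwarded to UI; damage and death only print, and a debug E key deals damage.
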(event OnHealthChanged(BPC_StatComponent)
  (params (CurrentHealth :type Integer) (CurrentMaxHealth :type Integer))
  ;[1 0.6128 0.2493] STAT EVENTS
  (Default|CallOnHealthChangedforUI CurrentHealth))

(event OnDamageTaken(BPC_StatComponent)
  ;[1 0.6128 0.2493] STAT EVENTS
  (Development|PrintString "Damaged"))

(event OnPlayerDied(BPC_StatComponent)
  ;[1 0.6128 0.2493] STAT EVENTS
  (Development|PrintString "Died"))

(event Custom|HandleFloatMovement
  ;[0 1 0.9333] Movement Logic
  (|HandleMovementLogic))

(event Input|EnhancedActionEvents|EnhancedInputActionIA_Drop
  (params (ActionValue :type Boolean) (ElapsedSeconds :type Float%20%28double-precision%29) (TriggeredSeconds :type Float%20%28double-precision%29) (InputAction :type Input%20Action%20Object%20Reference :default "/Game/Input/Actions/IA_Drop.IA_Drop"))
  ;[0 1 0.9188] Control Inputs
  (:Triggered
    (Variables|Default|SetbIsMovinDown true))
  (:Completed
    (Variables|Default|SetbIsMovinDown false)))

(event EventBeginPlay
  (Utilities|FlowControl|Sequence
    (:then_0
      (bind _aspc_player_controller (Utilities|Casting|CastToPC_PlayerController (Game|GetPlayerController 0)))
      (Input|AddMappingContext (PlayerController|LocalPlayerSubsystems|GetEnhancedInputLocalPlayerSubsystem _aspc_player_controller) "/Game/Input/IMC_Default.IMC_Default" 0 "(bIgnoreAllPressedKeysUntilRelease=True,bForceImmediately=False,bNotifyUserSettings=False)")
      (bind _returnvalue (Utilities|Time|SetTimerbyFunctionName 0 "HandleFloatMovement" (Variables|Default|GetTimer) true))
      (Variables|Default|SetTimerHandler _returnvalue))
    (:then_1
      (Default|InitHealth (Variables|Default|GetBPC_StatComponent)))))

(event Input|KeyboardEvents|DebugKeyE
  (params (Key :type Key%20Structure :default "None") (ActionValue :type Input%20Action%20Value%20Structure))
  ;[0.6198 0.008455 0] DEBUG AREA DO NOT TOUCH !!!
  (:Pressed
    (Default|DealDamage (Variables|Default|GetBPC_StatComponent) 1)))

(fn ConstructionScript)

(fn GetZChangeSpeed
  (params (Direction :type Float%20%28double-precision%29))
  (return (* (* (Variables|Default|GetAccelSpeed) Direction) (Variables|Default|GetTimer))))