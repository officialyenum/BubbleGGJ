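; AI enemy character that paces along the X axis, hurts players it touches and takes damage when hit from above.
; Walk and wall-check functions, apparently timer-driven, move it and reverse direction when it stays stuck; the ledge and wall traces are disconnected.
; Box overlaps send damage to Player-tagged characters, while capsule hits on the head feed BPC_StatComponent.
; The component's events drive a flicker on damage and delayed destruction on death.
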(event `self.ReceiveBeginPlay`
  ;[1 1 1] Start walk and health
  (`KismetSystemLibrary.K2_SetTimerDelegate` (`|CreateDelegate` :!event `Walk`) 0.01 true true)
  (`KismetSystemLibrary.K2_SetTimerDelegate` (`|CreateDelegate` :!event `Check wall and floor`) 0.333 true true)
  (`self.InitHealth` (`self.Health`)))

(event `/Game/Interfaces/ICombatInterface.DealDamage`
  (params (DamageAmount :type Integer))
  ;[1 1 1] Damage handling
  (`/Game/Characters/BPC_StatComponent.DealDamage` (`self.BPC_StatComponent`) DamageAmount))

(event `self.CapsuleComponent.OnComponentHit`
  (params (HitComponent :type "PrimitiveComponent Object Reference") (OtherActor :type "Actor Object Reference") (OtherComp :type "PrimitiveComponent Object Reference") (NormalImpulse :type "Vector Structure") (Hit :type "HitResult Structure (by ref)"))
  (bind (_bblockinghit _binitialoverlap _time _distance _location _impactpoint _normal _impactnormal) (`GameplayStatics.BreakHitResult` Hit))
  (bind (_returnvalue_x _returnvalue_y _returnvalue_z) (`KismetMathLibrary.BreakVector` (- _impactpoint (`self.K2_GetActorLocation`))))
  ;[1 1 1] when hit on head take damage
  (if (and (> _returnvalue_z 9.0) (< (.z _impactnormal) -0.5))
    (`/Game/Characters/BPC_StatComponent.DealDamage` (`self.BPC_StatComponent`) 1)
    (`KismetSystemLibrary.PrintString` "hurt")))

(event `self.BPC_StatComponent.OnPlayerDied`
  (`KismetSystemLibrary.Delay` 1.0)
  (`self.K2_DestroyActor`))

(event `self.BPC_StatComponent.OnDamageTaken`
  (`Timeline|Timeline` :!via `PlayFromStart`
    (:`Update`
      (`/Engine/EditorBlueprintResources/StandardMacros.FlipFlop`
        (:`A`
          (`self.SetActorHiddenInGame` true))
        (:`B`
          (`self.SetActorHiddenInGame` false))))
    (:`Finished`
      (`self.SetActorHiddenInGame` false)
      (`BlueprintMapLibrary.Map_Add` (`/Game/Characters/BPC_StatComponent.Stats` (`self.BPC_StatComponent`)) "NewEnumerator5"))))

(fn `ChangeWalkDirection`
  (set `self.WalkDirection` (* (`self.WalkDirection`) -1.0)))

(fn `Check wall and floor`
  (`|ExecutionSequence`
    (:`then_0`
      (if (<= (`KismetMathLibrary.VSize` (`self.GetVelocity`)) 0.0)
        (bind _result (`/Engine/EditorBlueprintResources/StandardMacros.IncrementInt` (`self.StuckCounter`))
          (:`  `
            (if (> _result (`self.StuckCheck`))
              (set `self.StuckCounter` 0)
              (`self.ChangeWalkDirection`))))
        (else
          (set `self.StuckCounter` 0))))
    (:`then_1`
      (for _array_element (`PrimitiveComponent.GetOverlappingActors` (`self.Box`) "/Script/Engine.Character")
        (if (`self.ActorHasTag` _array_element "Player")
          (message `/Game/Interfaces/ICombatInterface.DealDamage` _array_element 1)
          (`KismetSystemLibrary.PrintString` "Damage"))))))

(fn `InitHealth`
  (params (Health :type Integer))
  (bind _stats (`/Game/Characters/BPC_StatComponent.Stats` (`self.BPC_StatComponent`)))
  (`BlueprintMapLibrary.Map_Add` _stats "NewEnumerator1" Health)
  (`BlueprintMapLibrary.Map_Add` _stats "NewEnumerator2" Health))

(fn `UserConstructionScript`)

(fn `Walk`
  (`self.AddMovementInput` (`KismetMathLibrary.MakeVector` (`self.WalkDirection`))))