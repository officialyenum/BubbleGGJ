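; Player character for a 2D side-view game: a bubble that moves, jumps and switches between Default, Elastic and Heavy states.
; The state manager component drives animation and gravity; landing bounces Elastic, while Heavy slams with effects and velocity-scaled area damage to pawns.
; The stat component handles incoming damage, relaying health to UI, flickering the sprite and printing on death.
; Pause input asks the game mode to update the HUD.
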(event `self.BPC_StatComponent.OnHealthChanged`
  (params (CurrentHealth :type Integer) (CurrentMaxHealth :type Integer))
  ;[1 0.3902 0] Stats Events
  (`self.OnHealthChangedForUI` CurrentHealth))

(event `self.BPC_StatComponent.OnDamageTaken`
  ;[1 0.3902 0] Stats Events
  (bind _asabp_bubble (cast `/Game/Animations/ABP_Bubble` (`PaperZDAnimationComponent.AnimInstance` (`self.AnimationComponent`))))
  (set `/Game/Animations/ABP_Bubble.IsTakingDamage` true _asabp_bubble)
  (`self.FlickerSprite`))

(event `self.BPC_StatComponent.OnPlayerDied`
  ;[1 0.3902 0] Stats Events
  (`KismetSystemLibrary.PrintString` "You Died"))

(event `self.BPC_BubbleStateManager.OnStateChanged`
  (params (CurrentState :type "/Game/Data/Enums/EBubbleState Enum" :default "NewEnumerator0"))
  (bind _charactermovement (`self.CharacterMovement`))
  ;[1 0.3902 0] Stats Events
  ;;[1 1 1] Change State Animations or VFX Here
  (bind _asabp_bubble (cast `/Game/Animations/ABP_Bubble` (`PaperZDAnimationComponent.AnimInstance` (`self.AnimationComponent`))))
  (bind _output_get (set `/Game/Animations/ABP_Bubble.CurrentState` CurrentState _asabp_bubble))
  (switch `/Game/Data/Enums/EBubbleState` _output_get
    (:`NewEnumerator0`
      (set `CharacterMovementComponent.GravityScale` 2.0 _charactermovement :!label _label))
    (:`NewEnumerator1`
      (goto _label))
    (:`NewEnumerator2`
      (set `CharacterMovementComponent.GravityScale` 3.0 _charactermovement))))

(event `EnhancedInput|/Game/Input/Actions/IA_Move`
  (params (ActionValue :type "Float (double-precision)") (ElapsedSeconds :type "Float (double-precision)") (TriggeredSeconds :type "Float (double-precision)") (InputAction :type "InputAction Object Reference" :default "/Game/Input/Actions/IA_Move.IA_Move"))
  ;[0 0.09229 1] Input Area
  (:`Triggered`
    (`self.CanBubbleMove`
      (:`Can Move`
        (`self.UpdateDirection` ActionValue)
        (`self.AddMovementInput` (`KismetMathLibrary.MakeVector` 1.0) ActionValue)))))

(event `EnhancedInput|/Game/Input/Actions/IA_EnterDefaultState`
  (params (ActionValue :type Boolean) (ElapsedSeconds :type "Float (double-precision)") (TriggeredSeconds :type "Float (double-precision)") (InputAction :type "InputAction Object Reference" :default "/Game/Input/Actions/IA_EnterDefaultState.IA_EnterDefaultState"))
  ;[0 0.09229 1] Input Area
  ;;[1 0.006057 0] State Inputs
  (:`Started`
    (`/Game/Characters/BPC_BubbleStateManager.ChangeBubbleState` (`self.BPC_BubbleStateManager`) "NewEnumerator0")))

(event `EnhancedInput|/Game/Input/Actions/IA_EnterElasticState`
  (params (ActionValue :type Boolean) (ElapsedSeconds :type "Float (double-precision)") (TriggeredSeconds :type "Float (double-precision)") (InputAction :type "InputAction Object Reference" :default "/Game/Input/Actions/IA_EnterElasticState.IA_EnterElasticState"))
  ;[0 0.09229 1] Input Area
  ;;[1 0.006057 0] State Inputs
  (:`Started`
    (`/Game/Characters/BPC_BubbleStateManager.ChangeBubbleState` (`self.BPC_BubbleStateManager`) "NewEnumerator1")))

(event `EnhancedInput|/Game/Input/Actions/IA_Jump`
  (params (ActionValue :type Boolean) (ElapsedSeconds :type "Float (double-precision)") (TriggeredSeconds :type "Float (double-precision)") (InputAction :type "InputAction Object Reference" :default "/Game/Input/Actions/IA_Jump.IA_Jump"))
  ;[0 0.09229 1] Input Area
  (:`Triggered`
    (`self.CanBubbleJump`
      (:`Can Jump`
        (`self.Jump`))))
  (:`Completed`
    (`GameplayStatics.PlaySound2D` "/Game/Assets/sounds/Cues/bubble-pop-100784_Cue.bubble-pop-100784_Cue" 1.0 1.0 0.0 null null)
    (`self.StopJumping`)))

(event `EnhancedInput|/Game/Input/Actions/IA_EnterHeavyState`
  (params (ActionValue :type Boolean) (ElapsedSeconds :type "Float (double-precision)") (TriggeredSeconds :type "Float (double-precision)") (InputAction :type "InputAction Object Reference" :default "/Game/Input/Actions/IA_EnterHeavyState.IA_EnterHeavyState"))
  ;[0 0.09229 1] Input Area
  ;;[1 0.006057 0] State Inputs
  (:`Started`
    (`/Game/Characters/BPC_BubbleStateManager.ChangeBubbleState` (`self.BPC_BubbleStateManager`) "NewEnumerator2")))

(event `EnhancedInput|/Game/Input/Actions/IA_Pause`
  (params (ActionValue :type Boolean) (ElapsedSeconds :type "Float (double-precision)") (TriggeredSeconds :type "Float (double-precision)") (InputAction :type "InputAction Object Reference" :default "/Game/Input/Actions/IA_Pause.IA_Pause"))
  ;[0 0.09229 1] Input Area
  (:`Started`
    (bind _asbp_game_mode (cast `/Game/Game/BP_GameMode` (`GameplayStatics.GetGameMode`)))
    (if (`GameplayStatics.IsGamePaused`)
      (`/Game/Game/BP_GameMode.UpdateHUD` _asbp_game_mode "NewEnumerator5")
      (else
        (`/Game/Game/BP_GameMode.UpdateHUD` _asbp_game_mode "NewEnumerator2")))))

(event `self.OnLanded`
  (params (Hit :type "HitResult Structure (by ref)"))
  (bind _returnvalue (`self.K2_GetActorLocation`))
  (bind _bpc_bubblestatemanager (`self.BPC_BubbleStateManager`))
  (bind _returnvalue_2 (`KismetMathLibrary.Abs` (.z (`self.GetVelocity`))))
  ;[0.1269 1 0] Unreal In Built Event Listeners
  (`self.CanBounce`
    (:`Can Bounce`
      (`self.LaunchCharacter` (`KismetMathLibrary.MakeVector` 0.0 0.0 (+ _returnvalue_2 100.0)) false true)
      (bind _result (`/Engine/EditorBlueprintResources/StandardMacros.DecrementInt` (`self.bounceCounter`))
        (:`  `
          (if (<= _result 0)
            (`/Game/Characters/BPC_BubbleStateManager.ChangeBubbleState` (`self.BPC_BubbleStateManager`) "NewEnumerator0")
            (set `self.bounceCounter` 1)))))
    (:`It Is Heavy`
      (`NiagaraFunctionLibrary.SpawnSystemAtLocation` "/Game/Effects/SlamEffect.SlamEffect" _returnvalue (struct) (3.0 3.0 3.0))
      (`/Game/Characters/BPC_BubbleStateManager.ChangeBubbleState` _bpc_bubblestatemanager "NewEnumerator0")
      (bind _outhits (`KismetSystemLibrary.SphereTraceMultiForObjects` _returnvalue _returnvalue (`KismetMathLibrary.SafeDivide` _returnvalue_2 4.0) (`|MakeArray` "ObjectTypeQuery3" :!type "EObjectTypeQuery Enum") false (`|MakeArray` self :!type "Actor Object Reference") "None" true (struct :`R` 1.0 :`A` 1.0) (struct :`G` 1.0 :`A` 1.0) 2.0))
      (`GameplayStatics.SpawnEmitterAtLocation` null (`self.K2_GetActorLocation`))
      (`GameplayStatics.PlayWorldCameraShake` "/Game/Effects/CS_HeavyLandingFX.CS_HeavyLandingFX_C" (`self.K2_GetActorLocation`) 0.0 3000.0)
      (for _array_element _outhits
        (bind _damage (`/Game/Characters/BPC_StatComponent.GetDamageByState` (`self.BPC_StatComponent`) (`/Game/Characters/BPC_BubbleStateManager.GetBubbleState` _bpc_bubblestatemanager)))
        (message `/Game/Interfaces/ICombatInterface.DealDamage` (`.HitActor` (`GameplayStatics.BreakHitResult` _array_element)) _damage)))))

(event `/Game/Interfaces/ICombatInterface.DealDamage`
  (params (DamageAmount :type Integer))
  ;[1 0.3902 0] Interface Implementations
  (`/Game/Characters/BPC_StatComponent.DealDamage` (`self.BPC_StatComponent`) DamageAmount))

(event `FlickerSprite`
  (bind _sprite (`self.Sprite`))
  (bind (_spritecolor_r _spritecolor_g _spritecolor_b) (break `LinearColor` (`PaperFlipbookComponent.SpriteColor` _sprite)))
  ;[0.1269 1 0] Timeline Logic
  (bind _asabp_bubble (cast `/Game/Animations/ABP_Bubble` (`PaperZDAnimationComponent.AnimInstance` (`self.AnimationComponent`))))
  (if (`/Game/Animations/ABP_Bubble.IsTakingDamage` _asabp_bubble)
    (bind _returnvalue (`NiagaraFunctionLibrary.SpawnSystemAtLocation` "/Game/Effects/BasicAttackEnemyEffect.BasicAttackEnemyEffect" (`self.K2_GetActorLocation`)))
    (bind _returnvalue_2 (message `AnimationDataModel.GetPlayLength` _returnvalue))
    (`KismetSystemLibrary.Delay` _returnvalue_2)
    (bind (_direction _opacity) (`Timeline|Flicker Timeline` :!via `PlayFromStart`)
      (:`Update`
        (`PaperFlipbookComponent.SetSpriteColor` _sprite (`KismetMathLibrary.MakeColor` _spritecolor_r _spritecolor_g _spritecolor_b _opacity))))))

(fn `UpdateDirection`
  (params (Direction :type "Float (double-precision)"))
  (locals (CurrentRotation :type "Rotator Structure"))
  (set `local.CurrentRotation` (`Controller.GetControlRotation` (`self.GetController`)))
  (if (< (`local.Direction`) 0.0)
    (if (!= (.yaw (`local.CurrentRotation`)) 180.0)
      (`Controller.SetControlRotation` (`self.GetController`) (`KismetMathLibrary.MakeRotator` (.roll (`local.CurrentRotation`)) (.pitch (`local.CurrentRotation`)) 180.0)))
    (elif (!= (.yaw (`local.CurrentRotation`)) 0.0)
      (`Controller.SetControlRotation` (`self.GetController`) (`KismetMathLibrary.MakeRotator` (.roll (`local.CurrentRotation`)) (.pitch (`local.CurrentRotation`)))))))

(fn `UserConstructionScript`)