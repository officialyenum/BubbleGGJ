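; Game mode for a timed kill-all-enemies match, switching between menu, gameplay, pause, win and loss screens.
; On BeginPlay it gathers BP_AICharacters and tracks their destruction as a Kill Count quest in the quest manager component.
; UpdateHUD swaps widgets from a map, setting pause and input mode; entering Game starts a one-second countdown, also stored as a quest.
; Quest delegates rebroadcast progress and trigger victory, while timer expiry triggers defeat.
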(event `self.ReceiveBeginPlay`
  (`|ExecutionSequence`
    (:`then_0`
      ;[0.1269 1 0] Controller and HUD Initialized
      (bind _aspc_player_controller (cast `/Game/Controller/PC_PlayerController` (`GameplayStatics.GetPlayerController` 0)))
      (set `self.PlayerController` _aspc_player_controller)
      (`self.UpdateHUD` "NewEnumerator1"))
    (:`then_1`
      ;[1 0.006057 0] Init Enemy
      (`self.InitEnemyInLevel`))
    (:`then_2`
      ;[0.778 0.01124 1] Enemy Bind
      (for _array_element (`self.Enemies`)
        (add `self.OnDestroyed` _array_element (delegate `OnDestroyed_Event`))))))

(event `OnDestroyed_Event` :!signature `self.OnDestroyed`
  (params (DestroyedActor :type "Actor Object Reference"))
  ;[0.778 0.01124 1] Enemy Bind
  (bind _asbp_aicharacter (cast `/Game/Characters/BP_AICharacter` DestroyedActor))
  (`KismetArrayLibrary.Array_RemoveItem` (`self.Enemies`) _asbp_aicharacter)
  (bind _questitem (`/Game/Game/BPC_QuestManager.GetQuestByEnum` (`self.BPC_QuestManager`) "NewEnumerator1"))
  (`/Game/Game/BPC_QuestManager.UpdateAchievementByQuestEnum` (`self.BPC_QuestManager`) "NewEnumerator1" (+ (`.CurrentValue_9_D0CDB7204E3D98234704C5A68F73E4F2` (break `/Game/Data/Structs/SQuestItem` _questitem)) 1)))

(event `self.BPC_QuestManager.OnQuestAchievementUpdated`
  (params (QuestType :type "/Game/Data/Enums/EQuestType Enum" :default "NewEnumerator0") (QuestStruct :type "/Game/Data/Structs/SQuestItem Structure"))
  (bind (_title _currentvalue _condition _targetvalue) (break `/Game/Data/Structs/SQuestItem` QuestStruct))
  ;[1 0.3902 0] Quest Manager Delegates
  (switch `/Game/Data/Enums/EQuestType` QuestType
    (:`NewEnumerator1`
      (`self.OnEnemyLeftChanged` _currentvalue _targetvalue))
    (:`NewEnumerator2`
      (`self.OnTimerChanged` _currentvalue))))

(event `self.BPC_QuestManager.OnAllQuestAchieved`
  ;[1 0.3902 0] Quest Manager Delegates
  (`KismetSystemLibrary.PrintString` "All Quest Achieved Called" true true (struct :`R` 0.126865 :`G` 1.0 :`A` 1.0))
  (`self.UpdateHUD` "NewEnumerator3"))

(event `StartTimer`
  (if (not (`self.bIsTimerStarted`))
    (`/Game/Game/BPC_QuestManager.AddQuest` (`self.BPC_QuestManager`) "NewEnumerator2" (make `/Game/Data/Structs/SQuestItem` "Count Down" (`self.Timer`) "NewEnumerator3"))
    (bind _returnvalue (`KismetSystemLibrary.K2_SetTimerDelegate` (delegate `UpdateGameTime`) 1.0 true))
    (set `self.GameTimeHandler` _returnvalue)
    (set `self.bIsTimerStarted` true)))

(event `UpdateGameTime`
  (bind _bpc_questmanager (`self.BPC_QuestManager`))
  (bind _questitem (`/Game/Game/BPC_QuestManager.GetQuestByEnum` _bpc_questmanager "NewEnumerator2"))
  (bind _output_get (set `self.Timer` (- (`.CurrentValue_9_D0CDB7204E3D98234704C5A68F73E4F2` (break `/Game/Data/Structs/SQuestItem` _questitem)) 1)))
  (`/Game/Game/BPC_QuestManager.UpdateAchievementByQuestEnum` _bpc_questmanager "NewEnumerator2" _output_get)
  (if (<= (`self.Timer`) 0)
    (`self.UpdateHUD` "NewEnumerator4")))

(fn `GetEnemies`
  (returns (EnemiesKilled :type Integer) (TotalEnemies :type Integer))
  (bind _questitem (`/Game/Game/BPC_QuestManager.GetQuestByEnum` (`self.BPC_QuestManager`) "NewEnumerator1"))
  (bind (_title _currentvalue _condition _targetvalue) (break `/Game/Data/Structs/SQuestItem` _questitem))
  (return _currentvalue _targetvalue))

(fn `InitEnemyInLevel`
  (bind _bpc_questmanager (`self.BPC_QuestManager`))
  (bind _returnvalue (`KismetArrayLibrary.Array_Length` (`self.Enemies`)))
  (if (<= _returnvalue 0)
    (bind _outactors (`GameplayStatics.GetAllActorsOfClass` "/Game/Characters/BP_AICharacter.BP_AICharacter_C"))
    (bind _output_get (set `self.Enemies` _outactors))
    (`/Game/Game/BPC_QuestManager.AddQuest` _bpc_questmanager "NewEnumerator1" (make `/Game/Data/Structs/SQuestItem` "Kill Count" 0 "NewEnumerator3" (`KismetArrayLibrary.Array_Length` _output_get)))
    (bind _questitem (`/Game/Game/BPC_QuestManager.GetQuestByEnum` _bpc_questmanager "NewEnumerator1"))
    (bind (_title _currentvalue _condition _targetvalue) (break `/Game/Data/Structs/SQuestItem` _questitem))
    (`KismetSystemLibrary.PrintString` (`KismetStringLibrary.Concat_StrStr` "Total " (`KismetStringLibrary.Conv_IntToString` _targetvalue)))
    (`self.OnEnemyLeftChanged` _currentvalue _targetvalue)
    (else
      (`self.OnEnemyLeftChanged` 0 _returnvalue))))

(fn `UpdateHUD`
  (params (NewHud :type "/Game/Data/Enums/EHUDState Enum" :default "NewEnumerator1"))
  (bind _playercontroller (`self.PlayerController`))
  (bind (_value _returnvalue) (`BlueprintMapLibrary.Map_Find` (`self.Huds`) (`local.NewHud`)))
  (`/Engine/EditorBlueprintResources/StandardMacros.IsValid` (`self.CurrentHUD`)
    (:`Is Valid`
      (`Widget.RemoveFromParent` (`self.CurrentHUD`))
      (if (or (`KismetSystemLibrary.IsValidClass` _value) _returnvalue)
        (bind _returnvalue_2 (`|CreateWidget` _value (`self.PlayerController`) :!label _label))
        (bind _output_get (set `self.CurrentHUD` _returnvalue_2))
        (`UserWidget.AddToViewport` _output_get 0)
        (switch `/Game/Data/Enums/EHUDState` (`local.NewHud`)
          (:`NewEnumerator0`
            (set `PlayerController.bShowMouseCursor` true _playercontroller :!label _label_2)
            (`WidgetBlueprintLibrary.SetInputMode_GameAndUIEx` _playercontroller (`self.CurrentHUD`) "DoNotLock" false)
            (`GameplayStatics.SetGamePaused` true))
          (:`NewEnumerator1`
            (goto _label_2))
          (:`NewEnumerator5`
            (set `PlayerController.bShowMouseCursor` false _playercontroller)
            (`WidgetBlueprintLibrary.SetInputMode_GameOnly` _playercontroller)
            (`GameplayStatics.SetGamePaused` false)
            (`self.StartTimer`))
          (:`NewEnumerator2`
            (goto _label_2))
          (:`NewEnumerator3`
            (goto _label_2))
          (:`NewEnumerator4`
            (goto _label_2)))))
    (:`Is Not Valid`
      (goto _label))))

(fn `UserConstructionScript`)